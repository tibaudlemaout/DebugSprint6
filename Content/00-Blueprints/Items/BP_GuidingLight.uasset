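; BP_GuidingLight is a guiding light that shifts its point light color toward that of the nearest crystal.
; A looping timer, started one tick after BeginPlay, runs GetNearestCrystal every UpdateInterval.
; That function scans all actors of the Target class by distance, then lerps its light color a tenth of the way to the chosen crystal's, blending gradually over repeated updates.
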(event `self.ReceiveBeginPlay`
  (`KismetSystemLibrary.DelayUntilNextTick`)
  (`KismetSystemLibrary.K2_SetTimer` null "GetNearestCrystal" (`self.UpdateInterval`) true))

(fn `GetNearestCrystal`
  (locals (`Local Distance` :type "Float (single-precision)" :default 100000000.0) (`Local Crystal` :type "/Game/00-Blueprints/Items/BP_Item_Crystals Object Reference"))
  (bind _outactors (`GameplayStatics.GetAllActorsOfClass` (`self.Target`)))
  (for _array_element _outactors
    (bind _returnvalue (`self.GetDistanceTo` _array_element))
    (if (< _returnvalue (`local.Local Distance`))
      (set `local.Local Distance` _returnvalue)
      (set `local.Local Crystal` _array_element)))
  (`LightComponent.SetLightColor` (`self.PointLightComponent`) (`KismetMathLibrary.LinearColorLerp` (`LightComponentBase.GetLightColor` (`self.PointLightComponent`)) (`LightComponentBase.GetLightColor` (`/Game/00-Blueprints/Items/BP_Item_Crystals.PointLight` (`local.Local Crystal`))) 0.1) true))

(fn `UserConstructionScript`)