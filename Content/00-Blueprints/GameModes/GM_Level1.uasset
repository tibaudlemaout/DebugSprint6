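; GM_Level1 is the game mode for Level 1, which randomizes which crystal feeling type each crystal pedestal holds.
; On BeginPlay it shuffles an array of six E_CrystalsType values.
; It then assigns them by index to the FeelingType of every BP_Item_CrystalPedestre found in the level, so each pedestal gets a different type as long as there are no more than six.
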(event `self.ReceiveBeginPlay`
  (`self.RandomPedestalFeeling`))

(fn `RandomPedestalFeeling`
  (bind _output_get (set `self.FeelingArray` (`|MakeArray` (enumliteral `/Game/00-Blueprints/Enumerations/E_CrystalsType` "NewEnumerator0") "NewEnumerator1" "NewEnumerator2" "NewEnumerator3" "NewEnumerator4" "NewEnumerator5")))
  (`KismetArrayLibrary.Array_Shuffle` _output_get)
  (bind _outactors (`GameplayStatics.GetAllActorsOfClass` "/Game/00-Blueprints/Items/BP_Item_CrystalPedestre.BP_Item_CrystalPedestre_C"))
  (for (_array_element _array_index) _outactors
    (set `/Game/00-Blueprints/Items/BP_Item_CrystalPedestre.FeelingType` (`|GetArrayItem` (`self.FeelingArray`) _array_index) _array_element)))

(fn `UserConstructionScript`)